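; BP_MaterialEditor is a central controller for the dynamic floor's material settings, driving the look of every BP_Grid in the level.
; On BeginPlay it caches all grids after a zero-length Delay.
; Every Tick it pushes its variables into each grid's FloorMaterial as scalar and vector parameters, covering general blending, platform, wave and outline settings.
; The default outline color is hardcoded black rather than exposed through a variable.
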(event `self.ReceiveBeginPlay`
  (`KismetSystemLibrary.Delay` 0.0)
  (bind _outactors (`GameplayStatics.GetAllActorsOfClass` "/Game/DynamicFloor/Blueprints/BP_Grid.BP_Grid_C"))
  (set `self.Grids` _outactors))

(event `self.ReceiveTick`
  (params (DeltaSeconds :type "Float (single-precision)"))
  (`self.UpdateMaterialsOnGrids`))

(fn `UpdateMaterialsOnGrids`
  (locals (TempFloorMaterial :type "MaterialInstanceDynamic Object Reference"))
  (for _array_element (`self.Grids`)
    (set `local.TempFloorMaterial` (`/Game/DynamicFloor/Blueprints/BP_Grid.FloorMaterial` _array_element))
    (`|ExecutionSequence`
      (:`then_0`
        ;[1 1 1] GENERAL
        (`MaterialInstanceDynamic.SetScalarParameterValue` (`local.TempFloorMaterial`) "Smooth" (`KismetMathLibrary.Conv_BoolToDouble` (`self.IsSmooth`)))
        (`MaterialInstanceDynamic.SetScalarParameterValue` (`local.TempFloorMaterial`) "PlatformCombination" (`self.PlatformCombination`))
        (`MaterialInstanceDynamic.SetScalarParameterValue` (`local.TempFloorMaterial`) "InRadiusWaveMovement" (`self.InRadiusWaveMovement`))
        (`MaterialInstanceDynamic.SetScalarParameterValue` (`local.TempFloorMaterial`) "WaveCombination" (`self.WaveCombination`)))
      (:`then_1`
        ;[1 1 1] GENERAL OUTLINE
        (`MaterialInstanceDynamic.SetScalarParameterValue` (`local.TempFloorMaterial`) "InRadiusWaveHighlight" (`self.InRadiusWaveHighlight`))
        (`MaterialInstanceDynamic.SetScalarParameterValue` (`local.TempFloorMaterial`) "WaveCombinationHighlight" (`self.WaveCombinationHighlight`))
        (`MaterialInstanceDynamic.SetScalarParameterValue` (`local.TempFloorMaterial`) "PlatformCombinationHighlight" (`self.PlatformCombinationHighlight`))
        (`MaterialInstanceDynamic.SetScalarParameterValue` (`local.TempFloorMaterial`) "DefaultOutlineIntensity" (`self.DefaultOutlineIntensity`)))
      (:`then_2`
        ;[1 1 1] PLATFORM
        (`MaterialInstanceDynamic.SetScalarParameterValue` (`local.TempFloorMaterial`) "CollectionCount" (`KismetMathLibrary.Conv_IntToDouble` (`self.CollectionCount`)))
        (`MaterialInstanceDynamic.SetScalarParameterValue` (`local.TempFloorMaterial`) "Deadzone" (`self.Deadzone`))
        (`MaterialInstanceDynamic.SetScalarParameterValue` (`local.TempFloorMaterial`) "Radius" (`self.Radius`))
        (`MaterialInstanceDynamic.SetScalarParameterValue` (`local.TempFloorMaterial`) "Scale" (`self.Scale`)))
      (:`then_3`
        ;[1 1 1] PLATFORM OUTLINE
        (`MaterialInstanceDynamic.SetVectorParameterValue` (`local.TempFloorMaterial`) "PlatformOutlineColor" (`KismetMathLibrary.Conv_ColorToLinearColor` (`self.PlatformOutlineColor`)))
        (`MaterialInstanceDynamic.SetScalarParameterValue` (`local.TempFloorMaterial`) "PlatformOutlineIntensity" (`self.PlatformOutlineIntensity`)))
      (:`then_4`
        ;[1 1 1] Wave
        (`MaterialInstanceDynamic.SetScalarParameterValue` (`local.TempFloorMaterial`) "WaveCount" (`self.WaveCount`))
        (`MaterialInstanceDynamic.SetVectorParameterValue` (`local.TempFloorMaterial`) "WaveDirection" (`KismetMathLibrary.Conv_ColorToLinearColor` (`self.WaveDirection`)))
        (`MaterialInstanceDynamic.SetScalarParameterValue` (`local.TempFloorMaterial`) "WaveLength" (`self.WaveLength`))
        (`MaterialInstanceDynamic.SetVectorParameterValue` (`local.TempFloorMaterial`) "WaveOffset" (`KismetMathLibrary.Conv_VectorToLinearColor` (`self.WaveOffset`)))
        (`MaterialInstanceDynamic.SetScalarParameterValue` (`local.TempFloorMaterial`) "WaveSpeed" (`self.WaveSpeed`))
        (`MaterialInstanceDynamic.SetScalarParameterValue` (`local.TempFloorMaterial`) "WaveSteepness" (`self.WaveSteepness`)))
      (:`then_5`
        ;[1 1 1] WAVE OUTLINE
        (`MaterialInstanceDynamic.SetVectorParameterValue` :`self` (`local.TempFloorMaterial`) :`ParameterName` "DefaultOutlineColor")
        (`MaterialInstanceDynamic.SetScalarParameterValue` (`local.TempFloorMaterial`) "WaveOutlineAlphaAddition" (`self.WaveOutlineAlphaAddition`))))))

(fn `UserConstructionScript`)