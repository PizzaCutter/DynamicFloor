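; BP_Grid is a floor actor that lays out a grid of instanced static mesh cells.
; The construction script calls CreateGrid, whose nested loops over GridSize add instances spaced by CellSize and stretched vertically.
; On BeginPlay it creates a dynamic material instance from the mesh's first material and stores it as FloorMaterial; nothing in this graph drives its parameters.
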(event `self.ReceiveBeginPlay`
  (bind _instancedstaticmesh (`self.InstancedStaticMesh`))
  (bind _returnvalue (`PrimitiveComponent.CreateDynamicMaterialInstance` _instancedstaticmesh 0 (`PrimitiveComponent.GetMaterial` _instancedstaticmesh 0)))
  (set `self.FloorMaterial` _returnvalue))

(fn `CreateGrid`
  (locals (CurWidth :type Integer) (CurHeight :type Integer))
  (bind (_gridsize_x _gridsize_y) (`KismetMathLibrary.BreakVector2D` (`self.GridSize`)))
  (bind _gridsize_x_2 (`KismetMathLibrary.BreakVector2D` (`self.GridSize`)))
  (for _index (range (+ (`KismetMathLibrary.FTrunc` _gridsize_x_2) 1))
    (set `local.CurWidth` _index)
    (for _index_2 (range (+ (`KismetMathLibrary.FTrunc` _gridsize_y) 1))
      (set `local.CurHeight` _index_2)
      (`InstancedStaticMeshComponent.AddInstance` (`self.InstancedStaticMesh`) (`KismetMathLibrary.MakeTransform` (`KismetMathLibrary.MakeVector` (* (`local.CurWidth`) (`self.CellSize`)) (* (`local.CurHeight`) (`self.CellSize`))) (struct) (1.0 1.0 5.0))))))

(fn `UserConstructionScript`
  (`self.CreateGrid`))