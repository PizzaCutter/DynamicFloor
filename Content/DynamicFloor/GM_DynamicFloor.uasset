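; GM_DynamicFloor is a game mode that publishes world locations to the MPC_FloorWeights material parameter collection for a dynamic floor.
; Each Tick resets the write index and fills the numbered Position_ vector parameters with a far-away sentinel value.
; AddLocationToFloor writes a location into the next slot and advances the index, so locations must be resubmitted every frame.
; FloorWeights is resized on BeginPlay but not otherwise used here.
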(event `self.ReceiveBeginPlay`
  (`KismetArrayLibrary.Array_Resize` (`self.FloorWeights`) (`self.VectorParameterCount`)))

(event `self.ReceiveTick`
  (params (DeltaSeconds :type "Float (single-precision)"))
  (`self.ResetLocations`))

(fn `AddLocationToFloor`
  (params (LocationToAdd :type "Vector Structure"))
  (`KismetMaterialLibrary.SetVectorParameterValue` "/Game/DynamicFloor/Materials/MPC_FloorWeights.MPC_FloorWeights" (`KismetStringLibrary.Conv_StringToName` (`KismetStringLibrary.Concat_StrStr` "Position_" (`KismetStringLibrary.Conv_IntToString` (`self.CurIndex`)))) (`KismetMathLibrary.Conv_VectorToLinearColor` LocationToAdd))
  (`/Engine/EditorBlueprintResources/StandardMacros.IncrementInt` (`self.CurIndex`)))

(fn `ResetLocations`
  (set `self.CurIndex` 0)
  (for _index (range (+ (`self.VectorParameterCount`) 1))
    (`KismetMaterialLibrary.SetVectorParameterValue` "/Game/DynamicFloor/Materials/MPC_FloorWeights.MPC_FloorWeights" (`KismetStringLibrary.Conv_StringToName` (`KismetStringLibrary.Concat_StrStr` "Position_" (`KismetStringLibrary.Conv_IntToString` _index))) (make `LinearColor` -99999997952.0 -99999997952.0 -99999997952.0 -99999997952.0))))

(fn `UserConstructionScript`)